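; SMLPlayerControllerBP is a player controller Blueprint that manages the in-game escape and respawn menus.
; The menu input toggles the escape menu by checking widget validity, sharing its logic with explicit open and close events.
; Separate events open and close the respawn menu, printing debug strings.
; Opening either menu creates the widget and enables game-and-UI input with the cursor shown, while closing removes it and restores game-only input.
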(event EventBeginPlay)

(event EventTick
  (params (DeltaSeconds :type Float%20%28single-precision%29)))

(event EventCloseRespawnMenu
  (Development|PrintString "Respawn menu closed")
  (Input|SetInputModeGameOnly self)
  (Widget|RemovefromParent (Variables|Default|GetRespawnMenu))
  (Variables|Default|SetRespawnMenu 0)
  (Variables|Default|SetbShowMouseCursor false))

(event EventOpenRespawnMenu
  (bind _self self)
  (Development|PrintString "Respawn menu open")
  (bind _returnvalue (UserInterface|CreateWidget "/Game/Blueprints/RespawnMenu.RespawnMenu_C" _self _self))
  (bind _output_get (Variables|Default|SetRespawnMenu _returnvalue))
  (UserInterface|Viewport|AddtoViewport _output_get 0)
  (Input|SetInputModeGameandUI self _output_get "LockAlways" false)
  (Variables|Default|SetbShowMouseCursor true))

(event EventInputMenuPressed
  (bind _self self)
  (bind _escmenu (Variables|Default|GetEscMenu)
    (:then
      (Input|SetInputModeGameOnly self)
      (Widget|RemovefromParent _escmenu)
      (Variables|Default|SetEscMenu 0)
      (Variables|Default|SetbShowMouseCursor false))
    (:else
      (bind _returnvalue (UserInterface|CreateWidget "/Game/Blueprints/EscMenuInGame.EscMenuInGame_C" _self _self))
      (bind _output_get (Variables|Default|SetEscMenu _returnvalue))
      (UserInterface|Viewport|AddtoViewport _output_get 0)
      (Input|SetInputModeGameandUI self 0 "LockAlways" false)
      (Variables|Default|SetbShowMouseCursor true))))

(event EventCloseEscMenu
  (Input|SetInputModeGameOnly self)
  (Widget|RemovefromParent (stale EventInputMenuPressed _escmenu))
  (Variables|Default|SetEscMenu 0)
  (Variables|Default|SetbShowMouseCursor false))

(event EventOpenEscMenu
  (bind _self self)
  (bind _returnvalue (UserInterface|CreateWidget "/Game/Blueprints/EscMenuInGame.EscMenuInGame_C" _self _self))
  (bind _output_get (Variables|Default|SetEscMenu _returnvalue))
  (UserInterface|Viewport|AddtoViewport _output_get 0)
  (Input|SetInputModeGameandUI self 0 "LockAlways" false)
  (Variables|Default|SetbShowMouseCursor true))

(fn ConstructionScript)